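; Projectile actor for the TDCore game that flies straight along its forward vector at its Speed.
; On spawn it rolls a random Damage value, which nothing in this graph applies.
; Tick moves it with a swept location update and accumulates distance travelled, destroying it past a fixed range.
; It also destroys itself when its Cone component ends overlap with a TriggerVolume.
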(event `self.ReceiveBeginPlay`
  (set `self.Damage` (`KismetMathLibrary.RandomIntegerInRange` 20 50)))

(event `self.ReceiveTick`
  (params (DeltaSeconds :type "Float (single-precision)"))
  (bind _returnvalue (* DeltaSeconds (`self.Speed`)))
  (`self.K2_SetActorLocation` (+ (`self.K2_GetActorLocation`) (* (`self.GetActorForwardVector`) _returnvalue)) true)
  (bind _output_get (set `self.Length` (+ (`self.Length`) _returnvalue)))
  (if (>= _output_get 1000.0)
    (`self.K2_DestroyActor`)))

(event `self.Cone.OnComponentEndOverlap`
  (params (OverlappedComponent :type "PrimitiveComponent Object Reference") (OtherActor :type "Actor Object Reference") (OtherComp :type "PrimitiveComponent Object Reference") (OtherBodyIndex :type Integer))
  (cast `TriggerVolume` OtherActor)
  (`self.K2_DestroyActor`))

(fn `UserConstructionScript`)