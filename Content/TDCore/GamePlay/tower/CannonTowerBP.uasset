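; Cannon tower Blueprint that fires cannonball projectiles at a targeted monster.
; On FireBullet it gets its target and spawns a CannonBulletBP above its Cone component, rotated toward a point raised well above the monster's location.
; It then sets the projectile movement velocity along the bullet's forward vector at a fixed speed.
; Tick only calls the parent, and this graph does not show what triggers firing.
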(event `self.ReceiveTick`
  (params (DeltaSeconds :type "Float (single-precision)"))
  (`parent.ReceiveTick` DeltaSeconds))

(event `self.FireBullet`
  (bind _returnvalue (+ (`SceneComponent.K2_GetComponentLocation` (`self.Cone`)) (0.0 0.0 150.0)))
  (bind _monster (`self.GetTarget`))
  (bind _returnvalue_2 (`|SpawnActorFromClass` "/Game/TDCore/GamePlay/bullets/CannonBulletBP.CannonBulletBP_C" (`KismetMathLibrary.MakeTransform` _returnvalue (`KismetMathLibrary.FindLookAtRotation` _returnvalue (+ (`self.K2_GetActorLocation` _monster) (0.0 0.0 500.0)))) "Undefined" "OverrideRootScale" null null))
  (set `MovementComponent.Velocity` (* (`self.GetActorForwardVector` _returnvalue_2) 400) (`/Game/TDCore/GamePlay/bullets/CannonBulletBP.ProjectileMovement` _returnvalue_2)))

(fn `UserConstructionScript`
  (`parent.UserConstructionScript`))