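; Base tower actor for a tower defense game that turns toward and shoots BaseMonster enemies within range.
; Capsule overlap events keep a target list, and the first monster in it is the current target.
; Each tick the tower yaws toward that target with height ignored and counts down a cooldown.
; When ready, it spawns a BulletBP at its Cone component, aimed at the target, and resets the cooldown.
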(event `self.ReceiveTick`
  (params (DeltaSeconds :type "Float (single-precision)"))
  (`self.TryFaceToTarget`)
  (set `self.AttackRate` (- (`self.AttackRate`) DeltaSeconds))
  (`self.TryAttackTarget`))

(event `self.Capsule.OnComponentBeginOverlap`
  (params (OverlappedComponent :type "PrimitiveComponent Object Reference") (OtherActor :type "Actor Object Reference") (OtherComp :type "PrimitiveComponent Object Reference") (OtherBodyIndex :type Integer) (bFromSweep :type Boolean) (SweepResult :type "HitResult Structure (by ref)"))
  (bind _asbase_monster (cast `/Game/TDCore/GamePlay/monster/BaseMonster` OtherActor))
  (`KismetArrayLibrary.Array_AddUnique` (`self.targets`) _asbase_monster))

(event `self.Capsule.OnComponentEndOverlap`
  (params (OverlappedComponent :type "PrimitiveComponent Object Reference") (OtherActor :type "Actor Object Reference") (OtherComp :type "PrimitiveComponent Object Reference") (OtherBodyIndex :type Integer))
  (bind _asbase_monster (cast `/Game/TDCore/GamePlay/monster/BaseMonster` OtherActor))
  (`KismetArrayLibrary.Array_RemoveItem` (`self.targets`) _asbase_monster))

(fn `FireBullet`
  (bind _returnvalue (`SceneComponent.K2_GetComponentLocation` (`self.Cone`)))
  (bind _monster (`self.GetTarget`))
  (`|SpawnActorFromClass` "/Game/TDCore/GamePlay/bullets/BulletBP.BulletBP_C" (`KismetMathLibrary.MakeTransform` _returnvalue (`KismetMathLibrary.FindLookAtRotation` _returnvalue (`self.K2_GetActorLocation` _monster))) "Undefined" "OverrideRootScale" null null))

(fn `GetTarget`
  (returns (Monster :type "/Game/TDCore/GamePlay/monster/BaseMonster Object Reference") (IsValid :type Boolean))
  (locals (TempMonster :type "/Game/TDCore/GamePlay/monster/BaseMonster Object Reference"))
  (bind _targets (`self.targets`))
  (bind _returnvalue (> (`KismetArrayLibrary.Array_Length` _targets) 0))
  (if _returnvalue
    (bind _output_get (set `local.TempMonster` (`|GetArrayItem` _targets))))
  (return _output_get _returnvalue))

(fn `TryAttackTarget`
  (if (<= (`self.AttackRate`) 0.0)
    (bind (_monster _isvalid) (`self.GetTarget`))
    (if _isvalid
      (set `self.AttackRate` 1.0)
      (`self.FireBullet`))))

(fn `TryFaceToTarget`
  (bind (_monster _isvalid) (`self.GetTarget`))
  (if _isvalid
    (`self.K2_SetActorRotation` (`KismetMathLibrary.FindLookAtRotation` (`KismetMathLibrary.MakeVector` (.x (`self.K2_GetActorLocation`)) (.y (`self.K2_GetActorLocation`))) (`KismetMathLibrary.MakeVector` (.x (`self.K2_GetActorLocation` _monster)) (.y (`self.K2_GetActorLocation` _monster)))))))

(fn `UserConstructionScript`)